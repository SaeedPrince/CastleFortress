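; Behavior tree service that selects an opponent for an AI-controlled Paladin on each tick.
; It caches the generic AI controller and Paladin pawn, then passes the Paladin's seen-opponent list to PickATarget.
; PickATarget finds the nearest entry and writes its actor, location and health to the Blackboard.
; An invalid entry aborts the search; without a valid selection, it attempts list removal and clears target actor and health.
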(event `self.ReceiveTick`
  (params (OwnerActor :type "Actor Object Reference") (DeltaSeconds :type "Float (single-precision)"))
  (bind _targetactor (`self.TargetActor`))
  (bind _charref (`self.CharRef`))
  (bind _aiconref (`self.AICONRef`))
  (if (not (!= _aiconref null))
    (bind _asaicontroller_generic (cast `/Game/CastleFortress/Blueprints/GameMode/AIController_Generic` OwnerActor))
    (set `self.AICONRef` _asaicontroller_generic))
  (if (not (!= _charref null))
    (bind _ascharacter_paladin (cast `/Game/CastleFortress/Blueprints/GameMode/Character_Paladin` (`Controller.K2_GetPawn` _aiconref)))
    (set `self.CharRef` _ascharacter_paladin))
  (`/Engine/EditorBlueprintResources/StandardMacros.IsValid` (`BTFunctionLibrary.GetBlackboardValueAsActor` _targetactor)
    (:`Is Valid`
      _)
    (:`Is Not Valid`
      (`BTFunctionLibrary.SetBlackboardValueAsObject` _targetactor)))
  (`self.PickATarget` (`/Game/CastleFortress/Blueprints/GameMode/Character_Paladin.OpponentSeen` _charref) _charref))