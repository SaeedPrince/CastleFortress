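; BossFound is a Behavior Tree decorator that passes when the AI character has a valid PlayerSeen reference.
; Its condition check resolves the AI controller and character from the owner, then writes PlayerSeen to the BossActor blackboard key, clearing the key when nothing is seen.
; The check therefore updates the blackboard as a side effect of evaluating the condition.
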(fn `PerformConditionCheck`
  (params (OwnerActor :type "Actor Object Reference"))
  (returns (ReturnValue :type Boolean))
  (bind _output_get (set `self.AICnRef` (`/Game/CastleFortress/Blueprints/GameMode/AIFunctions.SetAIControllerRef` OwnerActor (`self.AICnRef`))))
  (bind _output_get_2 (set `self.CharRef` (`/Game/CastleFortress/Blueprints/GameMode/AIFunctions.SetCharacterRef` (`self.CharRef`) _output_get)))
  (bind _playerseen (`/Game/CastleFortress/Blueprints/GameMode/Character_Paladin.PlayerSeen` _output_get_2))
  (bind _returnvalue (!= _playerseen null))
  (if _returnvalue
    (`BTFunctionLibrary.SetBlackboardValueAsObject` (`self.BossActor`) _playerseen)
    (else
      (`BTFunctionLibrary.SetBlackboardValueAsObject` (`self.BossActor`))))
  (return _returnvalue))