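; NeedRotate is a behavior tree decorator that checks whether an AI-controlled Paladin character is facing its target.
; It lazily casts and caches the owning AIController_Generic and its controlled Character_Paladin.
; The condition reads the TargetActor location from the blackboard and returns IsCharacterFacingToActor using an acceptable-angle tolerance.
; Despite the asset's name, the raw result comes straight from the facing check without negation.
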(fn `PerformConditionCheck`
  (params (OwnerActor :type "Actor Object Reference"))
  (returns (ReturnValue :type Boolean))
  (bind _charref (`self.CharRef`))
  (bind _aiconref (`self.AIConRef`))
  (if (not (!= _aiconref null))
    (bind _asaicontroller_generic (cast `/Game/CastleFortress/Blueprints/GameMode/AIController_Generic` OwnerActor))
    (set `self.AIConRef` _asaicontroller_generic))
  (if (not (!= _charref null))
    (bind _ascharacter_paladin (cast `/Game/CastleFortress/Blueprints/GameMode/Character_Paladin` (`Controller.K2_GetPawn` _aiconref)))
    (set `self.CharRef` _ascharacter_paladin))
  (return (`/Game/CastleFortress/Blueprints/GameMode/CommonFunctions.IsCharacterFacingToActor` (`Actor.K2_GetActorLocation` (`BTFunctionLibrary.GetBlackboardValueAsActor` (`self.TargetActor`))) _charref (`self.AcceptableAngle`))))