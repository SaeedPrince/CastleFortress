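; Camera pawn for CastleFortress that moves according to axis input along a Forward or Right direction.
; The Move event takes a direction vector from the actor's yaw alone, so pitch and roll do not affect movement.
; It feeds that vector into AddMovementInput, scaling by the axis value and MoveTile with the sign inverted.
; A GetVector helper maps the direction choice to the rotator's forward or right vector.
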(event `Move`
  (params (AxisValue :type "Float (double-precision)") (Direction :type String))
  ;[1 1 0] Movement
  (bind _outvector (`/Game/CastleFortress/Blueprints/GameMode/CommonFunctions.GetMovementVector` (`KismetMathLibrary.MakeRotator` 0.0 0.0 (.yaw (`self.K2_GetActorRotation`))) Direction))
  (`self.AddMovementInput` _outvector (* AxisValue (`self.MoveTile`) -1.0)))

(fn `GetVector`
  (params (Rotator :type "Rotator Structure") (Direction :type String))
  (returns (Vector :type "Vector Structure"))
  (locals (OutVector :type "Vector Structure" :default (0.0 0.0 0.0)))
  (switch `string` Direction
    (:`Forward`
      (set `local.OutVector` (`KismetMathLibrary.GetForwardVector` Rotator)))
    (:`Right`
      (set `local.OutVector` (`KismetMathLibrary.GetRightVector` Rotator))))
  (return (`local.OutVector`)))

(fn `UserConstructionScript`)