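; Behavior tree task that makes an AI Paladin fight its blackboard target, reacting to that opponent's state.
; SetGameObjects caches the AI controller and pawn, reads the target actor and flags when none is valid.
; Depending on the target Paladin's state, the controller either attacks once, if not already attacking, or defends using the target's fire turn and look-up.
; The task finishes immediately after issuing the action, without waiting for it to complete.
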(event `self.ReceiveExecute`
  (params (OwnerActor :type "Actor Object Reference"))
  (bind _aicnref (`self.AICnRef`))
  (bind _notargetfound (`self.SetGameObjects` OwnerActor true true false true))
  (if (not _notargetfound)
    (bind _ascharacter_paladin (cast `/Game/CastleFortress/Blueprints/GameMode/Character_Paladin` (`self.CurrentTarget`)))
    (switch `int` (`/Game/CastleFortress/Blueprints/GameMode/Character_Paladin.State` _ascharacter_paladin)
      (:`0`
        (if (not (`/Game/CastleFortress/Blueprints/GameMode/Character_Paladin.IsAttacking` (`self.CharRef`))) :!label _label
          (`/Game/CastleFortress/Blueprints/GameMode/AIController_Generic.AttackOnce` _aicnref)))
      (:`1`
        (`/Game/CastleFortress/Blueprints/GameMode/AIController_Generic.Defend` _aicnref (`/Game/CastleFortress/Blueprints/GameMode/Character_Paladin.FireTurn` _ascharacter_paladin) (`/Game/CastleFortress/Blueprints/GameMode/Character_Paladin.FireLookUp` _ascharacter_paladin) :!label _label_2))
      (:`2`
        (goto _label_2))
      (:`3`
        (goto _label))
      (:`4`
        (goto _label))
      (:`5`
        (goto _label)))
    (bind _output_get (set `self.Success` true)))
  (`self.FinishExecute` _output_get))