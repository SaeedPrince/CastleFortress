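; GameState for the Castle Fortress mode that periodically announces how many allies and enemies remain.
; BeginPlay starts a looping timer at the AnouncePeriod interval, which calls AnounceStats by name.
; AnounceStats prints the AllyRemained and EnemyRemained counts on screen without logging them; nothing in these graphs updates either count.
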(event `self.ReceiveBeginPlay`
  ;[0 1 0] Anounce function starts
  (`KismetSystemLibrary.K2_SetTimer` self "AnounceStats" (`self.AnouncePeriod`) true))

(fn `AnounceStats`
  (`KismetSystemLibrary.PrintString` (`KismetStringLibrary.Concat_StrStr` "Allies remained: " (`KismetStringLibrary.Conv_IntToString` (`self.AllyRemained`))) true false (struct :`G` 0.66 :`B` 1.0 :`A` 1.0) 5.0)
  (`KismetSystemLibrary.PrintString` (`KismetStringLibrary.Concat_StrStr` "Enemies remained: " (`KismetStringLibrary.Conv_IntToString` (`self.EnemyRemained`))) true false (struct :`G` 0.66 :`B` 1.0 :`A` 1.0) 5.0))

(fn `UserConstructionScript`)