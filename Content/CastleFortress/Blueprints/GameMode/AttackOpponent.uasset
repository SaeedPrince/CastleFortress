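; Behavior tree task that makes an AI-controlled Paladin attack by calling Attack on its generic AI controller.
; On execute it casts and caches the controller and its controlled character, then delegates the attack to the controller.
; Older in-task logic for random aim offsets and timed attack animation messages is left disconnected.
; FinishExecute is also unwired, so the task never reports completion itself.
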(event `self.ReceiveExecute`
  (params (OwnerActor :type "Actor Object Reference"))
  (bind _aiconref (`self.AIConRef`))
  (if (not (!= _aiconref null))
    (bind _asaicontroller_generic (cast `/Game/CastleFortress/Blueprints/GameMode/AIController_Generic` OwnerActor))
    (bind _output_get (set `self.AIConRef` _asaicontroller_generic)))
  (if (not (!= (`self.CharRef`) null))
    (bind _ascharacter_paladin (cast `/Game/CastleFortress/Blueprints/GameMode/Character_Paladin` (`Controller.K2_GetPawn` _aiconref)))
    (bind _output_get_2 (set `self.CharRef` _ascharacter_paladin)))
  (`/Game/CastleFortress/Blueprints/GameMode/AIController_Generic.Attack` _output_get))

(fn `EndAttackPose`
  (message `/Game/Caladan/Blueprint/MyInterface.InterfaceAttackPoseEnd` (`SkeletalMeshComponent.GetAnimInstance` (`Character.Mesh` (`self.CharRef`)))))