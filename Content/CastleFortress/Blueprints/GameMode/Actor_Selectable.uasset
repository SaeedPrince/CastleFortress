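; Actor_Selectable is an actor that responds to mouse hover and clicks on its static mesh.
; On BeginPlay it caches the first player controller as PlayerController_Camera.
; Hover events use that reference to switch the cursor to crosshairs and back to default.
; Clicking only prints the pressed button's display name, with no selection logic yet.
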(event `self.ReceiveBeginPlay`
  ;[0 1 0] Assigning controller reference
  (bind _asplayer_controller_camera (cast `/Game/CastleFortress/Blueprints/GameMode/PlayerController_Camera` (`GameplayStatics.GetPlayerController` 0)))
  (set `self.ControllerRef` _asplayer_controller_camera))

(event `self.StaticMesh.OnBeginCursorOver`
  (params (TouchedComponent :type "PrimitiveComponent Object Reference"))
  ;[0 1 0] Mouse Cursor Change During Mouse Over
  (set `PlayerController.CurrentMouseCursor` "Crosshairs" (`self.ControllerRef`)))

(event `self.StaticMesh.OnEndCursorOver`
  (params (TouchedComponent :type "PrimitiveComponent Object Reference"))
  ;[0 1 0] Mouse Cursor Change During Mouse Over
  (set `PlayerController.CurrentMouseCursor` "Default" (`self.ControllerRef`)))

(event `self.StaticMesh.OnClicked`
  (params (TouchedComponent :type "PrimitiveComponent Object Reference") (ButtonPressed :type "Key Structure"))
  ;[1 1 0] Action
  (`KismetSystemLibrary.PrintString` (`KismetTextLibrary.Conv_TextToString` (`KismetInputLibrary.Key_GetDisplayName` ButtonPressed))))

(fn `UserConstructionScript`)