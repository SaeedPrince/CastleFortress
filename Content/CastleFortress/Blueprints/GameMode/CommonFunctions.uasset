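; Blueprint library of small math helpers in the CastleFortress GameMode folder.
; GetMovementVector returns a rotator's forward or right vector according to a direction selector.
; MakeRotatorByZ keeps only the yaw of a rotator and zeroes pitch and roll.
; AFloatPowerBInt computes an integer power of a float by multiplying into an output value in a countdown loop, with no explicit initialization of that value in the graph.
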(fn `AFloatPowerBInt`
  (params (InputA :type "Float (double-precision)") (InputB :type Integer))
  (returns (OutputFloat :type "Float (double-precision)"))
  (locals (OutFloat :type "Float (double-precision)" :default 1.0) (Counter :type Integer))
  (bind _output_get (set `local.Counter` InputB))
  (while (> _output_get 0)
    (set `local.OutFloat` (* InputA (`local.OutFloat`)))
    (set `local.Counter` (- (`local.Counter`) 1)))
  (return (`local.OutFloat`)))

(fn `GetMovementVector`
  (params (Rotator :type "Rotator Structure") (Direction :type String))
  (returns (OutVector :type "Vector Structure"))
  (locals (OutVect :type "Vector Structure"))
  (switch `string` Direction
    (:`Forward`
      (set `local.OutVect` (`KismetMathLibrary.GetForwardVector` Rotator)))
    (:`Right`
      (set `local.OutVect` (`KismetMathLibrary.GetRightVector` Rotator))))
  (return (`local.OutVect`)))

(fn `MakeRotatorByZ`
  (params (InputRotator :type "Rotator Structure"))
  (returns (OutputRotator :type "Rotator Structure"))
  (return (`KismetMathLibrary.MakeRotator` 0.0 0.0 (.yaw InputRotator))))