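; Behavior tree task that sends an AI-controlled Paladin character toward a location stored in the blackboard.
; On execute it lazily casts and caches the owning generic AI controller and its controlled Paladin pawn.
; It passes the Destination key's vector to the character's MoveToDestination, then finishes successfully right away without checking for arrival.
; A failed cast stops execution before the task reports finishing.
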(event `self.ReceiveExecute`
  (params (OwnerActor :type "Actor Object Reference"))
  (if (not (!= (`self.AIConRef`) null))
    (bind _asaicontroller_generic (cast `/Game/CastleFortress/Blueprints/GameMode/AIController_Generic` OwnerActor))
    (bind _output_get (set `self.AIConRef` _asaicontroller_generic)))
  (if (not (!= (`self.CharRef`) null))
    (bind _ascharacter_paladin (cast `/Game/CastleFortress/Blueprints/GameMode/Character_Paladin` (`Controller.K2_GetPawn` _output_get)))
    (bind _output_get_2 (set `self.CharRef` _ascharacter_paladin)))
  (`/Game/CastleFortress/Blueprints/GameMode/Character_Paladin.MoveToDestination` _output_get_2 (`BTFunctionLibrary.GetBlackboardValueAsVector` (`self.Destination`)))
  (`self.FinishExecute` true))