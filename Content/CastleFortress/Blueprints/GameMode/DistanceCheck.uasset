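; Behavior tree tick node, apparently a service, that checks the controlled Paladin's distance to its TargetActor for AI movement.
; Each tick it lazily caches the generic AI controller and its Character_Paladin pawn, stopping if either cast fails.
; It passes the target's location to the Paladin's FarAwayXY function and writes the results to the NeedMove and Movement blackboard keys.
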(event `self.ReceiveTick`
  (params (OwnerActor :type "Actor Object Reference") (DeltaSeconds :type "Float (single-precision)"))
  (bind _aiconref (`self.AICONRef`))
  (if (not (!= _aiconref null))
    (bind _asaicontroller_generic (cast `/Game/CastleFortress/Blueprints/GameMode/AIController_Generic` OwnerActor))
    (set `self.AICONRef` _asaicontroller_generic))
  (if (not (!= (`self.CharRef`) null))
    (bind _ascharacter_paladin (cast `/Game/CastleFortress/Blueprints/GameMode/Character_Paladin` (`Controller.K2_GetPawn` _aiconref)))
    (bind _output_get (set `self.CharRef` _ascharacter_paladin)))
  (bind (_outputbool _movement) (`/Game/CastleFortress/Blueprints/GameMode/Character_Paladin.FarAwayXY` _output_get (`Actor.K2_GetActorLocation` (`BTFunctionLibrary.GetBlackboardValueAsActor` (`self.TargetActor`)))))
  (`BTFunctionLibrary.SetBlackboardValueAsBool` (`self.NeedMove`) _outputbool)
  (`BTFunctionLibrary.SetBlackboardValueAsVector` (`self.Movement`) _movement))