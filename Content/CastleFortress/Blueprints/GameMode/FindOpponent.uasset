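; Behavior tree tick node that targets the closest opponent seen by an AI-controlled Paladin.
; It lazily caches the AIController_Generic and its Character_Paladin, then scans OpponentSeen by distance, removing invalid entries and printing the count.
; The selected opponent's actor and location go to the blackboard; TargetActor is cleared when none is selected.
; Distance and SelectedOpponent are never reset here between ticks.
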(event `self.ReceiveTick`
  (params (OwnerActor :type "Actor Object Reference") (DeltaSeconds :type "Float (single-precision)"))
  (bind _charref (`self.CharRef`))
  (bind _distance (`self.Distance`))
  (bind _selectedopponent (`self.SelectedOpponent`))
  (bind _targetactor (`self.TargetActor`))
  (bind _aiconref (`self.AICONRef`))
  (bind _opponentseen (`/Game/CastleFortress/Blueprints/GameMode/Character_Paladin.OpponentSeen` _charref))
  (bind _output (`|GetArrayItem` _opponentseen _selectedopponent))
  (if (not (!= _aiconref null))
    (bind _asaicontroller_generic (cast `/Game/CastleFortress/Blueprints/GameMode/AIController_Generic` OwnerActor))
    (set `self.AICONRef` _asaicontroller_generic))
  (if (not (!= _charref null))
    (bind _ascharacter_paladin (cast `/Game/CastleFortress/Blueprints/GameMode/Character_Paladin` (`Controller.K2_GetPawn` _aiconref)))
    (set `self.CharRef` _ascharacter_paladin))
  (`KismetSystemLibrary.PrintString` (`KismetStringLibrary.Conv_IntToString` (`KismetArrayLibrary.Array_Length` _opponentseen)) true true (struct :`G` 0.66 :`B` 1.0 :`A` 1.0) 8.0)
  (for (_array_element _array_index) _opponentseen
    (if (!= _array_element null)
      (if (== _distance 0.0)
        (bind _returnvalue (`KismetMathLibrary.VSize` (- (`Actor.K2_GetActorLocation` _array_element) (`Actor.K2_GetActorLocation` _charref))))
        (set `self.Distance` _returnvalue :!label _label)
        (set `self.SelectedOpponent` _array_index)
        (elif (< _returnvalue _distance)
          (goto _label)))
      (else
        (`KismetArrayLibrary.Array_RemoveItem` _opponentseen _array_element))))
  (if (!= _selectedopponent -1)
    (`BTFunctionLibrary.SetBlackboardValueAsObject` _targetactor _output)
    (`BTFunctionLibrary.SetBlackboardValueAsVector` (`self.TargetLocation`) (`Actor.K2_GetActorLocation` _output))
    (else
      (`BTFunctionLibrary.SetBlackboardValueAsObject` _targetactor))))