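; CloseEnough is a behavior tree decorator that gates AI branches on the distance between the controlled pawn and a blackboard target actor.
; It casts its owner to AIController_Generic, then measures the straight-line distance from that controller's pawn to the TargetActor blackboard value.
; Despite its name, the condition passes when that distance is at or beyond AcceptableDistance, not within it.
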(fn `PerformConditionCheck`
  (params (OwnerActor :type "Actor Object Reference"))
  (returns (ReturnValue :type Boolean))
  (bind _asaicontroller_generic (cast `/Game/CastleFortress/Blueprints/GameMode/AIController_Generic` OwnerActor))
  (set `self.AIConRef` _asaicontroller_generic)
  (return (>= (`KismetMathLibrary.VSize` (- (`Actor.K2_GetActorLocation` (`BTFunctionLibrary.GetBlackboardValueAsActor` (`self.TargetActor`))) (`Actor.K2_GetActorLocation` (`Controller.K2_GetPawn` (`self.AIConRef`))))) (`self.AcceptableDistance`))))