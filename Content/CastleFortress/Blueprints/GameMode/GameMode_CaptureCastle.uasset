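; Game mode for the Capture Castle mode that populates the match with ally and enemy AI when play begins.
; BeginPlay runs the parent logic, then loops through the StartAlly and StartEnemy arrays, passing each entry to AddAIAtLocation.
; Leftover unconnected nodes for single-index spawns and an index debug print never run.
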(event `self.ReceiveBeginPlay`
  (`parent.ReceiveBeginPlay`)
  (for _array_element (`self.StartAlly`)
    (`self.AddAIAtLocation` _array_element))
  (for (_array_element_2 _array_index) (`self.StartEnemy`)
    (`self.AddAIAtLocation` _array_element_2)))

(fn `UserConstructionScript`
  (`parent.UserConstructionScript`))