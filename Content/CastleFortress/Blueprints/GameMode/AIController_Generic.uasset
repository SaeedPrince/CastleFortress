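; Generic AI controller that drives a character's movement, turning and repeated attacks through CharRef.
; AssignBlackboard stores home location and the pawn, then runs the attacker tree for Ally paladins or the defender tree for Enemy ones.
; AttackStart begins a looping timer whose AttackController replays the attack pose while the stored TargetHealth stays positive.
; Separate timers call the character's functions that end each pose and execution; AttackStop cancels the loop.
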(event `MoveDirectly`
  (params (WorldDirection :type "Vector Structure"))
  ;[0 1 0] Character Movement
  (`/Game/CastleFortress/Blueprints/GameMode/Character_Paladin.MoveDirectly` (`self.CharRef`) WorldDirection))

(event `MoveByInput`
  (params (AxisValue :type "Float (double-precision)") (Direction :type String))
  ;[0.5 0.5 0.5] Character movement Obsolete
  (`/Game/CastleFortress/Blueprints/GameMode/Character_Paladin.MoveByInput` (`self.CharRef`) AxisValue Direction))

(event `TurnByInput`
  (params (AxisValue :type "Float (double-precision)"))
  ;[0 1 0] Turn character
  (`/Game/CastleFortress/Blueprints/GameMode/Character_Paladin.TurnByInput` (`self.CharRef`) AxisValue))

(event `AttackStop`
  (bind _timerattackcontroller (`self.TimerAttackController`))
  ;[1 1 0] Attack
  (if (`KismetSystemLibrary.K2_TimerExistsHandle` _timerattackcontroller)
    (`KismetSystemLibrary.K2_ClearAndInvalidateTimerHandle` _timerattackcontroller)))

(event `AttackStart`
  (params (TargetHealth :type "Float (double-precision)"))
  ;[1 1 0] Attack
  (if (and (> TargetHealth 0.0) (not (`KismetSystemLibrary.K2_TimerExistsHandle` (`self.TimerAttackController`))))
    (`|ExecutionSequence`
      (:`then_0`
        (set `self.TargetHealth` TargetHealth)
        (`/Game/CastleFortress/Blueprints/GameMode/Character_Paladin.AttackPoseStart` (`self.CharRef`)))
      (:`then_1`
        (bind _returnvalue (`KismetSystemLibrary.K2_SetTimer` self "AttackController" (`self.AttackDuration`) true))
        (set `self.TimerAttackController` _returnvalue))
      (:`then_2`
        (`self.SetEndAttackPoseTimer`)))))

(event `SetEndAttackPoseTimer`
  ;[1 1 0] Attack
  (`KismetSystemLibrary.K2_SetTimer` (`self.CharRef`) "EndAttackPose" (`self.AttackPoseDuration`))
  (`KismetSystemLibrary.K2_SetTimer` (`self.CharRef`) "EndAttackExe" (`self.AttackExeDuration`)))

(fn `AssignBlackboard`
  (bind _returnvalue (`self.K2_GetPawn`))
  (bind _returnvalue_2 (`AIBlueprintHelperLibrary.GetBlackboard` self))
  (`self.UseBlackboard` "/Game/CastleFortress/Blueprints/GameMode/Blackboard_Generic.Blackboard_Generic")
  (`BlackboardComponent.SetValueAsVector` _returnvalue_2 "HomeLocation" (`self.K2_GetActorLocation` _returnvalue))
  (`BlackboardComponent.SetValueAsObject` _returnvalue_2 "SelfActor" _returnvalue)
  (bind _ascharacter_paladin (cast `/Game/CastleFortress/Blueprints/GameMode/Character_Paladin` _returnvalue))
  (switch `string` (`/Game/CastleFortress/Blueprints/GameMode/Character_Paladin.Type` _ascharacter_paladin)
    (:`Ally`
      (`self.RunBehaviorTree` "/Game/CastleFortress/Blueprints/GameMode/BTreeAttackers.BTreeAttackers"))
    (:`Enemy`
      (`self.RunBehaviorTree` "/Game/CastleFortress/Blueprints/GameMode/BTreeDefenders.BTreeDefenders"))))

(fn `AttackController`
  (if (> (`self.TargetHealth`) 0.0)
    (`|ExecutionSequence`
      (:`then_0`
        (`/Game/CastleFortress/Blueprints/GameMode/Character_Paladin.AttackPoseStart` (`self.CharRef`)))
      (:`then_1`
        (`self.SetEndAttackPoseTimer`)))
    (else
      (`KismetSystemLibrary.K2_ClearAndInvalidateTimerHandle` (`self.TimerAttackController`)))))

(fn `UserConstructionScript`)