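; AIFunctions is a set of helper functions that resolve AI controller and character references.
; Each returns the passed-in reference if it is set, acting as a lazy cache that casts only when needed.
; SetAIControllerRef otherwise casts the owner actor to AIController_Generic.
; SetCharacterRef otherwise casts the controller's controlled pawn to Character_Paladin, tying that lookup to the Paladin class.
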(fn `SetAIControllerRef`
  (params (OwnerActor :type "Actor Object Reference") (AIControllerRef :type "/Game/CastleFortress/Blueprints/GameMode/AIController_Generic Object Reference"))
  (returns (AIController :type "/Game/CastleFortress/Blueprints/GameMode/AIController_Generic Object Reference"))
  (locals (LocalAiController :type "/Game/CastleFortress/Blueprints/GameMode/AIController_Generic Object Reference"))
  (if (!= AIControllerRef null)
    (set `local.LocalAiController` AIControllerRef)
    (else
      (bind _asaicontroller_generic (cast `/Game/CastleFortress/Blueprints/GameMode/AIController_Generic` OwnerActor))
      (set `local.LocalAiController` _asaicontroller_generic)))
  (return (`local.LocalAiController`)))

(fn `SetCharacterRef`
  (params (CharacterRef :type "/Game/CastleFortress/Blueprints/GameMode/Character_Paladin Object Reference") (AIControllerRef :type "/Game/CastleFortress/Blueprints/GameMode/AIController_Generic Object Reference"))
  (returns (Character :type "/Game/CastleFortress/Blueprints/GameMode/Character_Paladin Object Reference"))
  (locals (LocalCharacter :type "/Game/CastleFortress/Blueprints/GameMode/Character_Paladin Object Reference"))
  (if (!= CharacterRef null)
    (set `local.LocalCharacter` CharacterRef)
    (else
      (bind _ascharacter_paladin (cast `/Game/CastleFortress/Blueprints/GameMode/Character_Paladin` (`Controller.K2_GetPawn` AIControllerRef)))
      (set `local.LocalCharacter` _ascharacter_paladin)))
  (return (`local.LocalCharacter`)))