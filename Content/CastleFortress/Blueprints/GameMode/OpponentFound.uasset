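; Behavior Tree decorator that checks whether an AI character has an opponent to target, returning the BossFound flag.
; It starts from the blackboard's TargetActor, then scans the character's OpponentSeen list for the nearest opponent, removing invalid entries.
; SetTarget raises BossFound and writes the target, distance and location to the blackboard, plus state and health for Paladin targets.
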(fn `PerformConditionCheck`
  (params (OwnerActor :type "Actor Object Reference"))
  (returns (ReturnValue :type Boolean))
  (bind _currenttarget (`self.CurrentTarget`))
  (bind _selfactor (`self.SelfActor`))
  (bind _charref (`self.CharRef`))
  (bind _returnvalue (`BTFunctionLibrary.GetBlackboardValueAsActor` (`self.TargetActor`)))
  (bind _opponentseen (`/Game/CastleFortress/Blueprints/GameMode/Character_Paladin.OpponentSeen` _charref))
  (bind _output_get (set `self.AICnRef` (`/Game/CastleFortress/Blueprints/GameMode/AIFunctions.SetAIControllerRef` OwnerActor (`self.AICnRef`))))
  (set `self.CharRef` (`/Game/CastleFortress/Blueprints/GameMode/AIFunctions.SetCharacterRef` _charref _output_get))
  (if (not (!= (`BTFunctionLibrary.GetBlackboardValueAsActor` _selfactor) null))
    (`BTFunctionLibrary.SetBlackboardValueAsObject` _selfactor _charref))
  (if (!= _returnvalue null)
    (`self.SetTarget` _returnvalue))
  (for _array_element _opponentseen
    (`/Engine/EditorBlueprintResources/StandardMacros.IsValid` _array_element
      (:`Is Valid`
        (`/Engine/EditorBlueprintResources/StandardMacros.IsValid` _currenttarget
          (:`Is Valid`
            (if (< (`/Game/CastleFortress/Blueprints/GameMode/CommonFunctions.DestinationBetweenTwoActors` _array_element _charref) (`/Game/CastleFortress/Blueprints/GameMode/CommonFunctions.DestinationBetweenTwoActors` _currenttarget _charref))
              (`self.SetTarget` _array_element)))
          (:`Is Not Valid`
            (`self.SetTarget` _array_element))))
      (:`Is Not Valid`
        (`KismetArrayLibrary.Array_RemoveItem` _opponentseen _array_element))))
  (return (`self.BossFound`)))