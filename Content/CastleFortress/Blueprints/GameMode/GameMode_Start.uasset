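; Game mode for a castle battle that registers spawn points and spawns Ally and Enemy paladin AI.
; BeginPlay or GameStart sorts PlayerStarts into player, ally and enemy references by object name, then links itself to the camera controller.
; AddAI spawns a paladin at a random team start, possesses it with a new generic AI controller, assigns its blackboard and tints its shield by team.
; The player paladin spawn macro is never called.
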(event `self.ReceiveBeginPlay`
  ;[0 1 0] Begin Play
  (`self.MacSetPlayerStartRefs` :!label _label)
  (`self.MacSetGameObjects`))

(event `GameStart`
  ;[0 1 0] Begin Play
  (goto _label))

(event `AddAI`
  (params (Type :type String))
  ;[0 1 0] Add AI
  (switch `string` Type
    (:`Ally`
      (`self.MacAddAI` "Ally" (`self.AllyArray`) (`self.StartAlly`) 1.0))
    (:`Enemy`
      (`self.MacAddAI` "Enemy" (`self.EnemyArray`) (`self.StartEnemy`) 0.0 1.0))))

(fn `UserConstructionScript`)