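; Game mode for the Fortress mode that spawns allied and enemy AI.
; On BeginPlay it registers itself on GameState_Fortress, then starts a looping SpawnAI timer at SpawnAIPeriod.
; SpawnAI adds Ally and Enemy pairs until SpawnNumber reaches zero.
; The counter is not reset here, so later timer ticks spawn nothing unless it is refilled elsewhere.
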(event `self.ReceiveBeginPlay`
  (`parent.ReceiveBeginPlay`)
  (bind _asgame_state_fortress (cast `/Game/CastleFortress/Blueprints/GameMode/GameState_Fortress` (`GameplayStatics.GetGameState`)))
  (set `/Game/CastleFortress/Blueprints/GameMode/GameState_Fortress.GameModeRef` self _asgame_state_fortress)
  (`KismetSystemLibrary.K2_SetTimer` self "SpawnAI" (`self.SpawnAIPeriod`) true))

(fn `SpawnAI`
  (locals (SpawnNumber :type Integer :default 3))
  (bind _spawnnumber (`local.SpawnNumber`))
  (while (> _spawnnumber 0)
    (`self.AddAI` "Ally")
    (`self.AddAI` "Enemy")
    (set `local.SpawnNumber` (- _spawnnumber 1))))

(fn `UserConstructionScript`
  (`parent.UserConstructionScript`))