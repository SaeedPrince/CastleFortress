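; Base game state for Castle Fortress that tracks remaining allies and enemies and decides victory or defeat.
; On BeginPlay, looping timers periodically show and, after an offset delay, hide an announcement widget with both counts.
; A one-second end check declares Defeat when allies run out, otherwise Victory when enemies do, then clears the timers and passes the message to GameInstance_Generic to end the game.
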(event `self.ReceiveBeginPlay`
  ;[0 1 0] Anounce function starts
  (bind _asgame_mode_generic (cast `/Game/CastleFortress/Blueprints/GameModes/GameMode_Generic` (`GameplayStatics.GetGameMode`)))
  (set `self.GameModeRef` _asgame_mode_generic)
  (bind _returnvalue (`KismetSystemLibrary.K2_SetTimer` self "AnounceShow" (`self.AnouncePeriod`) true))
  (set `self.TimerAnounceShow` _returnvalue)
  (`KismetSystemLibrary.Delay` (`self.AnounceShowTime`))
  (bind _returnvalue_2 (`KismetSystemLibrary.K2_SetTimer` self "AnounceHide" (`self.AnouncePeriod`) true))
  (set `self.TimerAnounceHide` _returnvalue_2)
  (bind _returnvalue_3 (`KismetSystemLibrary.K2_SetTimer` self "EndCheck" 1.0 true))
  (set `self.TimerEndCheck` _returnvalue_3))

(fn `AnounceHide`
  (bind _widgetrefanounce (`self.WidgetRefAnounce`))
  (`/Engine/EditorBlueprintResources/StandardMacros.IsValid` _widgetrefanounce
    (:`Is Valid`
      (`Widget.RemoveFromParent` _widgetrefanounce))))

(fn `AnounceShow`
  (bind _widgetrefanounce (`self.WidgetRefAnounce`))
  (`/Engine/EditorBlueprintResources/StandardMacros.IsValid` _widgetrefanounce
    (:`Is Valid`
      _)
    (:`Is Not Valid`
      (bind _returnvalue (`|CreateWidget` "/Game/CastleFortress/Blueprints/Widgets/AnounceStats.AnounceStats_C" (`GameplayStatics.GetPlayerController` 0)))
      (set `self.WidgetRefAnounce` _returnvalue)))
  (`TextBlock.SetText` (`/Game/CastleFortress/Blueprints/Widgets/AnounceStats.txtAllyRemain` _widgetrefanounce) (`KismetTextLibrary.Conv_IntToText` (`self.AllyRemained`)))
  (`TextBlock.SetText` (`/Game/CastleFortress/Blueprints/Widgets/AnounceStats.txtEnemyRemain` _widgetrefanounce) (`KismetTextLibrary.Conv_IntToText` (`self.EnemyRemained`)))
  (`UserWidget.AddToViewport` _widgetrefanounce 0))

(fn `EndCheck`
  (locals (Message :type Text :default "Defeat"))
  (if (<= (`self.AllyRemained`) 0)
    (set `local.Message` "Defeat")
    (`|ExecutionSequence` :!label _label
      (:`then_0`
        (`KismetSystemLibrary.K2_ClearAndInvalidateTimerHandle` (`self.TimerAnounceShow`))
        (`KismetSystemLibrary.K2_ClearAndInvalidateTimerHandle` (`self.TimerAnounceHide`))
        (`KismetSystemLibrary.K2_ClearAndInvalidateTimerHandle` (`self.TimerEndCheck`))
        (`self.AnounceHide`))
      (:`then_1`
        (bind _asgame_instance_generic (cast `/Game/CastleFortress/Blueprints/GameInstances/GameInstance_Generic` (`GameplayStatics.GetGameInstance`)))
        (set `/Game/CastleFortress/Blueprints/GameInstances/GameInstance_Generic.Message` (`local.Message`) _asgame_instance_generic)
        (`/Game/CastleFortress/Blueprints/GameInstances/GameInstance_Generic.EndGame` _asgame_instance_generic)))
    (elif (<= (`self.EnemyRemained`) 0)
      (set `local.Message` "Victory")
      (goto _label))))

(fn `UserConstructionScript`)