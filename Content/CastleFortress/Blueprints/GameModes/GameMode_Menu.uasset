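; GameMode_Menu is the menu game mode that shows an end-game message screen when play begins.
; On BeginPlay it casts the game instance to GameInstance_Generic, stopping if the cast fails.
; It creates the EndGame widget if none exists, copies the instance's Message into its text, and adds it to the viewport.
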(event `self.ReceiveBeginPlay`
  (bind _widgetrefendgame (`self.WidgetRefEndGame`))
  (bind _asgame_instance_generic (cast `/Game/CastleFortress/Blueprints/GameInstances/GameInstance_Generic` (`GameplayStatics.GetGameInstance`)))
  (`/Engine/EditorBlueprintResources/StandardMacros.IsValid` _widgetrefendgame
    (:`Is Valid`
      _)
    (:`Is Not Valid`
      (bind _returnvalue (`|CreateWidget` "/Game/CastleFortress/Blueprints/Widgets/EndGame.EndGame_C" (`GameplayStatics.GetPlayerController` 0)))
      (set `self.WidgetRefEndGame` _returnvalue)))
  (`TextBlock.SetText` (`/Game/CastleFortress/Blueprints/Widgets/EndGame.txtMessage` _widgetrefendgame) (`/Game/CastleFortress/Blueprints/GameInstances/GameInstance_Generic.Message` _asgame_instance_generic))
  (`UserWidget.AddToViewport` _widgetrefendgame 0))

(fn `UserConstructionScript`)