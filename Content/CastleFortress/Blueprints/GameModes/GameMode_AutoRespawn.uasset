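; GameMode_AutoRespawn is a game mode that keeps adding Ally and Enemy AI throughout play.
; On BeginPlay it runs the parent logic, then starts a looping timer that calls SpawnAI every SpawnAIPeriod.
; Each SpawnAI call loops SpawnCount times, calling AddAIRandom once per side, so both teams receive equal waves with no check on living AI in this graph.
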(event `self.ReceiveBeginPlay`
  (`parent.ReceiveBeginPlay`)
  (`KismetSystemLibrary.K2_SetTimer` self "SpawnAI" (`self.SpawnAIPeriod`) true))

(fn `SpawnAI`
  (locals (SpawnNumber :type Integer :default 3))
  (bind _spawnnumber (`local.SpawnNumber`))
  (set `local.SpawnNumber` (`self.SpawnCount`))
  (while (> _spawnnumber 0)
    (`self.AddAIRandom` "Ally")
    (`self.AddAIRandom` "Enemy")
    (set `local.SpawnNumber` (- _spawnnumber 1))))

(fn `UserConstructionScript`
  (`parent.UserConstructionScript`))