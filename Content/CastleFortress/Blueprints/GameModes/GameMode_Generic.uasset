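; Castle Fortress game mode that spawns the player's Paladin and adds Ally attacker or Enemy defender AI Paladins on request.
; BeginPlay sorts PlayerStarts by object-name substring, caches game state and controller, then spawns and possesses the player as an Ally.
; AI events spawn at random or given starts, deriving behavior tree, array and shield color from team.
; Each AI gets a manually spawned controller; every spawn increments its team's remaining count in GameState.
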(event `self.ReceiveBeginPlay`
  ;[0 1 0] Begin Play
  (`|ExecutionSequence`
    (:`then_0`
      (`self.MacSetPlayerStartRefs`))
    (:`then_1`
      (`self.MacSetGameObjects`))
    (:`then_2`
      (`self.MacStartPlayer`))))

(event `AddAIRandom`
  (params (Type :type String))
  (bind (_bttreeref _pawnarrayref _redvalue _greenvalue) (`self.GetAIAttributes` Type))
  (bind (_location _rotation) (`self.GetRandomLocation` (`self.GetStartArray` Type)))
  ;[1 1 0] Add random AI
  (`self.MacAddAnAI` "/Game/CastleFortress/Blueprints/Characters/Paladin_AI.Paladin_AI_C" _bttreeref _location _rotation _pawnarrayref Type _redvalue _greenvalue)
  (`self.UpdateGameState` Type))

(event `AddAIAtLocation`
  (params (PlayerStart :type "PlayerStart Object Reference"))
  (bind _type (`self.GetPlayerStartType` PlayerStart))
  (bind (_location _rotation) (`self.GetLocation` PlayerStart))
  (bind (_bttreeref _pawnarrayref _redvalue _greenvalue) (`self.GetAIAttributes` _type))
  ;[1 1 0] Add AI at location
  (`self.MacAddAnAI` "/Game/CastleFortress/Blueprints/Characters/Paladin_AI.Paladin_AI_C" _bttreeref _location _rotation _pawnarrayref _type _redvalue _greenvalue)
  (`self.UpdateGameState` _type))

(fn `GetAIAttributes`
  (params (Type :type String))
  (returns (BtTreeRef :type "BehaviorTree Object Reference") (PawnArrayRef :type "Array of /Game/CastleFortress/Blueprints/Characters/Paladin_AI Object Reference") (RedValue :type "Float (double-precision)") (GreenValue :type "Float (double-precision)"))
  (locals (LocalBtTree :type "BehaviorTree Object Reference") (LocalPawnArray :type "Array of /Game/CastleFortress/Blueprints/Characters/Paladin_AI Object Reference") (LocalRedValue :type "Float (double-precision)" :default 0.0) (LocalGreenValue :type "Float (double-precision)" :default 0.0) (LocalStartArray :type "Array of PlayerStart Object Reference"))
  (switch `string` Type
    (:`Ally`
      (set `local.LocalBtTree` "/Game/CastleFortress/Blueprints/AI/BTreeAttackers.BTreeAttackers")
      (set `local.LocalPawnArray` (`self.AllyArray`))
      (set `local.LocalRedValue` 0.0)
      (set `local.LocalGreenValue` 1.0))
    (:`Enemy`
      (set `local.LocalBtTree` "/Game/CastleFortress/Blueprints/AI/BTreeDefenders.BTreeDefenders")
      (set `local.LocalPawnArray` (`self.EnemyArray`))
      (set `local.LocalRedValue` 1.0)
      (set `local.LocalGreenValue` 0.0)))
  (return (`local.LocalBtTree`) (`local.LocalPawnArray`) (`local.LocalRedValue`) (`local.LocalGreenValue`)))

(fn `GetLocation`
  (params (PlayerStart :type "Actor Object Reference"))
  (returns (Location :type "Vector Structure") (Rotation :type "Rotator Structure"))
  (return (.location (`self.GetTransform` PlayerStart)) (.rotation (`self.GetTransform` PlayerStart))))

(fn `GetPlayerStartType`
  (params (PlayerStart :type "PlayerStart Object Reference"))
  (returns (Type :type String))
  (locals (OutputType :type String))
  (bind _returnvalue (`KismetSystemLibrary.GetObjectName` PlayerStart))
  (if (`KismetStringLibrary.Contains` _returnvalue "Player")
    (set `local.OutputType` "Player")
    (elif (`KismetStringLibrary.Contains` _returnvalue "Ally")
      (set `local.OutputType` "Ally")
      (elif (`KismetStringLibrary.Contains` _returnvalue "Enemy")
        (bind _output_get (set `local.OutputType` "Enemy")))))
  (return _output_get))

(fn `GetRandomLocation`
  (params (StartArray :type "Array of PlayerStart Object Reference"))
  (returns (Location :type "Vector Structure") (Rotation :type "Rotator Structure"))
  (bind (_location _rotation) (`self.GetLocation` (`|GetArrayItem` StartArray (`KismetMathLibrary.RandomIntegerInRange` 0 (- (`KismetArrayLibrary.Array_Length` StartArray) 1)))))
  (return _location _rotation))

(fn `GetStartArray`
  (params (Type :type String))
  (returns (StartArray :type "Array of PlayerStart Object Reference"))
  (locals (LocalStartArray :type "Array of PlayerStart Object Reference"))
  (switch `string` Type
    (:`Ally`
      (set `local.LocalStartArray` (`self.StartAlly`)))
    (:`Enemy`
      (set `local.LocalStartArray` (`self.StartEnemy`))))
  (return (`local.LocalStartArray`)))

(fn `UpdateGameState`
  (params (Type :type String))
  (bind _gamestateref (`self.GameStateRef`))
  (switch `string` Type
    (:`Ally`
      (set `/Game/CastleFortress/Blueprints/GameStates/GameState_Generic.AllyRemained` (+ (`/Game/CastleFortress/Blueprints/GameStates/GameState_Generic.AllyRemained` _gamestateref) 1) _gamestateref))
    (:`Enemy`
      (set `/Game/CastleFortress/Blueprints/GameStates/GameState_Generic.EnemyRemained` (+ (`/Game/CastleFortress/Blueprints/GameStates/GameState_Generic.EnemyRemained` _gamestateref) 1) _gamestateref))))

(fn `UserConstructionScript`)