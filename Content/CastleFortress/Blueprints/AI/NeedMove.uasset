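; NeedMove is a behavior tree decorator that checks whether an AI pawn is still too far from its target.
; It reads the TargetActor blackboard key and, if that actor is valid, casts the owner to AIController_Generic to get the controlled pawn.
; It passes when the straight-line distance between pawn and target exceeds AcceptableDistance.
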(fn `PerformConditionCheck`
  (params (OwnerActor :type "Actor Object Reference"))
  (returns (ReturnValue :type Boolean))
  (bind _returnvalue (`BTFunctionLibrary.GetBlackboardValueAsActor` (`self.TargetActor`)))
  (`/Engine/EditorBlueprintResources/StandardMacros.IsValid` _returnvalue
    (:`Is Valid`
      (bind _asaicontroller_generic (cast `/Game/CastleFortress/Blueprints/Controllers/AIController_Generic` OwnerActor))
      (set `self.AIConRef` _asaicontroller_generic)
      (return (> (`KismetMathLibrary.VSize` (- (`Actor.K2_GetActorLocation` _returnvalue) (`Actor.K2_GetActorLocation` (`Controller.K2_GetPawn` (`self.AIConRef`))))) (`self.AcceptableDistance`))))))