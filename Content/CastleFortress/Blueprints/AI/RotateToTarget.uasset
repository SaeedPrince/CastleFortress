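; Behavior tree task that turns an AI-controlled Paladin character to face its target actor.
; It casts the owner to AIController_Generic, caches it, then reads the target actor from the blackboard.
; The target's location and an acceptable angle go to the Paladin's FaceToDestination, and the task then reports success.
; A failed cast stops execution without finishing the task.
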(event `self.ReceiveExecute`
  (params (OwnerActor :type "Actor Object Reference"))
  (if (not (!= (`self.AIConRef`) null))
    (bind _asaicontroller_generic (cast `/Game/CastleFortress/Blueprints/Controllers/AIController_Generic` OwnerActor))
    (bind _output_get (set `self.AIConRef` _asaicontroller_generic)))
  (bind _ascharacter_paladin (cast `/Game/CastleFortress/Blueprints/Characters/Character_Paladin` (`Controller.K2_GetPawn` _output_get)))
  (`/Game/CastleFortress/Blueprints/Characters/Character_Paladin.FaceToDestination` _ascharacter_paladin (`Actor.K2_GetActorLocation` (`BTFunctionLibrary.GetBlackboardValueAsActor` (`self.TargetActor`))) (`self.AcceptableAngle`))
  (`self.FinishExecute` true))