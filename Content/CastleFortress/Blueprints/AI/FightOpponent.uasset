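; Behavior tree task that makes an AI fighter react to the combat state of its target Paladin.
; SetGameObjects caches the controller and pawn and reads the target from the blackboard, ending the task if none exists.
; A switch on the target's state has the controller defend using lookup arrays indexed by the opponent's FireIndex, flank around its location, or, for all other states, attack once.
; Busy flags prevent repeating an action already underway.
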(event `self.ReceiveExecute`
  (params (OwnerActor :type "Actor Object Reference"))
  (bind _aicnref (`self.AICnRef`))
  (bind _charref (`self.CharRef`))
  (bind _currenttarget (`self.CurrentTarget`))
  (bind _returnvalue (`KismetSystemLibrary.GetObjectName` _charref))
  (bind _notargetfound (`self.SetGameObjects` OwnerActor true true false true))
  (if _notargetfound
    (`self.FinishExecute` (`self.Success`) :!label _label)
    (else
      (bind _ascharacter_paladin (cast `/Game/CastleFortress/Blueprints/Characters/Character_Paladin` _currenttarget))
      (switch `int` (`/Game/CastleFortress/Blueprints/Characters/Character_Paladin.State` _ascharacter_paladin)
        (:`0`
          (if (not (`/Game/CastleFortress/Blueprints/Characters/Character_Paladin.IsAttacking` _charref)) :!label _label_2
            _
            (else
              (set `self.Success` true :!label _label_3)
              (goto _label))))
        (:`1`
          (if (not (`/Game/CastleFortress/Blueprints/Characters/Character_Paladin.IsDefending` _charref))
            (`KismetSystemLibrary.PrintString` (`KismetStringLibrary.Concat_StrStr` _returnvalue " Defending") true true (struct :`B` 1.0 :`A` 1.0))
            (bind (_newx _newy) (`self.TheOpposite` (`/Game/CastleFortress/Blueprints/Characters/Character_Paladin.FireIndex` _ascharacter_paladin)))
            (`/Game/CastleFortress/Blueprints/Controllers/AIController_Generic.Defend` _aicnref _newx _newy)
            (goto _label_3)
            (else
              (goto _label_3))))
        (:`2`
          (if (not (`/Game/CastleFortress/Blueprints/Characters/Character_Paladin.IsFlanking` _charref))
            (`KismetSystemLibrary.PrintString` (`KismetStringLibrary.Concat_StrStr` _returnvalue " Flanking") true true (struct :`G` 1.0 :`A` 1.0))
            (`/Game/CastleFortress/Blueprints/Controllers/AIController_Generic.Flank` _aicnref (`Actor.K2_GetActorLocation` _currenttarget) (`self.FlankAngel`) (`self.AcceptableAngle`))
            (goto _label_3)
            (else
              (goto _label_3))))
        (:`3`
          (goto _label_2))
        (:`4`
          (goto _label_2))
        (:`5`
          (goto _label_2))
        (:`6`
          (goto _label_2))
        (:`7`
          (goto _label_2)))
      (`KismetSystemLibrary.PrintString` (`KismetStringLibrary.Concat_StrStr` _returnvalue " Attacking") true true (struct :`R` 1.0 :`A` 1.0))
      (`/Game/CastleFortress/Blueprints/Controllers/AIController_Generic.AttackOnce` _aicnref)
      (`MiniTimer.MiniTimer` 0.0))))

(fn `TheOpposite`
  (params (FireIndex :type Integer))
  (returns (NewX :type "Float (double-precision)") (NewY :type "Float (double-precision)"))
  (locals (XArray :type "Array of Float (double-precision)") (YArray :type "Array of Float (double-precision)"))
  (return (`|GetArrayItem` (`local.XArray`) FireIndex) (`|GetArrayItem` (`local.YArray`) FireIndex)))