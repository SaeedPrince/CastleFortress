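; Behavior tree task that turns the AI-controlled Paladin to face its blackboard target actor in Castle Fortress.
; It caches the generic AI controller on first run, then passes the pawn and target location to a FacePawnToLocation latent action with configurable angle, interval and end time.
; The task finishes when that action completes and aborts when the target actor is invalid.
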(event `self.ReceiveExecute`
  (params (OwnerActor :type "Actor Object Reference"))
  (bind _returnvalue (`BTFunctionLibrary.GetBlackboardValueAsActor` (`self.TargetActor`)))
  (if (not (!= (`self.AIConRef`) null))
    (bind _asaicontroller_generic (cast `/Game/CastleFortress/Blueprints/Controllers/AIController_Generic` OwnerActor))
    (bind _output_get (set `self.AIConRef` _asaicontroller_generic)))
  (bind _ascharacter_paladin (cast `/Game/CastleFortress/Blueprints/Characters/Character_Paladin` (`Controller.K2_GetPawn` _output_get)))
  (`/Engine/EditorBlueprintResources/StandardMacros.IsValid` _returnvalue
    (:`Is Valid`
      (bind _success (`FacePawnToLocation.FacePawnToLocation` _ascharacter_paladin (`Actor.K2_GetActorLocation` _returnvalue) (`self.AcceptableAngle`) (`self.TInterval`) (`self.ETime`))
        (:`Finished`
          (`self.FinishExecute` _success))))
    (:`Is Not Valid`
      (`self.FinishAbort`))))