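; Behavior tree decorator that checks whether a Paladin AI has an opponent to target.
; It caches the controller and pawn, reads the blackboard target, then scans the pawn's OpponentSeen list, switching to closer opponents and removing invalid entries.
; SetTarget writes the chosen actor, distance, location, state and health to the blackboard, so the condition check also updates targeting data as a side effect.
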(fn `PerformConditionCheck`
  (params (OwnerActor :type "Actor Object Reference"))
  (returns (ReturnValue :type Boolean))
  (bind _currenttarget (`self.CurrentTarget`))
  (bind _charref (`self.CharRef`))
  (bind _returnvalue (`BTFunctionLibrary.GetBlackboardValueAsActor` (`self.TargetActor`)))
  (bind _opponentseen (`/Game/CastleFortress/Blueprints/Characters/Character_Paladin.OpponentSeen` _charref))
  (`self.SetGameObjects` OwnerActor true true true)
  (if (!= _returnvalue null)
    (`self.SetTarget` _returnvalue))
  (set `self.OpponentFound` false)
  (for _array_element _opponentseen
    (`/Engine/EditorBlueprintResources/StandardMacros.IsValid` _array_element
      (:`Is Valid`
        (`/Engine/EditorBlueprintResources/StandardMacros.IsValid` _currenttarget
          (:`Is Valid`
            (set `self.OpponentFound` true)
            (if (< (`/Game/CastleFortress/Blueprints/Libraries/CommonFunctions.DestinationBetweenTwoActors` _array_element _charref) (`/Game/CastleFortress/Blueprints/Libraries/CommonFunctions.DestinationBetweenTwoActors` _currenttarget _charref))
              (`self.SetTarget` _array_element)))
          (:`Is Not Valid`
            (`self.SetTarget` _array_element))))
      (:`Is Not Valid`
        (`KismetArrayLibrary.Array_RemoveItem` _opponentseen _array_element))))
  (return (`self.OpponentFound`)))