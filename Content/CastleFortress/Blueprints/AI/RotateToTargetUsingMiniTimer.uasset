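; Behavior tree task that turns the AI-controlled Paladin character toward the target actor stored in the blackboard.
; SetGameObjects caches the controller, character and current target, then a MiniTimer drives step-wise turning at a set interval over a set duration.
; Each update recomputes turn direction within an acceptable angle.
; When the timer finishes, the task reports success if a turn is still needed and failure otherwise.
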(event `self.ReceiveExecute`
  (params (OwnerActor :type "Actor Object Reference"))
  (bind _charref (`self.CharRef`))
  (bind _acceptableangle (`self.AcceptableAngle`))
  (bind _returnvalue (`Actor.K2_GetActorLocation` (`self.CurrentTarget`)))
  (`self.SetGameObjects` OwnerActor true true false true)
  (`MiniTimer.MiniTimer` (`self.RotateInterval`) (`self.RotateDuration`)
    (:`Update`
      (`/Game/CastleFortress/Blueprints/Characters/Character_Paladin.TurnOnePoint` _charref (`/Game/CastleFortress/Blueprints/Libraries/CommonFunctions.CharacterTurnWiseToFaceToActor` _returnvalue _charref _acceptableangle)))
    (:`Finished`
      (if (`/Game/CastleFortress/Blueprints/Libraries/CommonFunctions.IsCharacterNeedTurn` _returnvalue _charref _acceptableangle)
        (`self.FinishExecute` true)
        (else
          (`self.FinishExecute` false))))))