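; Behavior Tree task that sends the AI-controlled Paladin toward the actor stored in the TargetActor blackboard key.
; On execute it caches the owning AIController_Generic, then passes the target's current location to MoveToDestination on the controlled Character_Paladin.
; It finishes successfully right after that call, and never calls FinishExecute if the target is invalid or a cast fails.
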(event `self.ReceiveExecute`
  (params (OwnerActor :type "Actor Object Reference"))
  (bind _returnvalue (`BTFunctionLibrary.GetBlackboardValueAsActor` (`self.TargetActor`)))
  (if (not (!= (`self.AIConRef`) null))
    (bind _asaicontroller_generic (cast `/Game/CastleFortress/Blueprints/Controllers/AIController_Generic` OwnerActor))
    (bind _output_get (set `self.AIConRef` _asaicontroller_generic)))
  (`/Engine/EditorBlueprintResources/StandardMacros.IsValid` _returnvalue
    (:`Is Valid`
      (bind _ascharacter_paladin (cast `/Game/CastleFortress/Blueprints/Characters/Character_Paladin` (`Controller.K2_GetPawn` _output_get)))
      (`/Game/CastleFortress/Blueprints/Characters/Character_Paladin.MoveToDestination` _ascharacter_paladin (`Actor.K2_GetActorLocation` _returnvalue))
      (`self.FinishExecute` true))))