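; Behavior Tree task that starts or stops an AI-controlled Paladin's attack on its current opponent.
; On execute it caches the generic AI controller and its Paladin pawn, then checks the blackboard target actor.
; A valid target passes its health to the controller's AttackStart, otherwise AttackStop is called, and the task finishes successfully.
; A separate EndAttackPose function sends an attack-pose-end interface message to the Paladin's anim instance.
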(event `self.ReceiveExecute`
  (params (OwnerActor :type "Actor Object Reference"))
  (bind _aiconref (`self.AIConRef`))
  (if (not (!= _aiconref null))
    (bind _asaicontroller_generic (cast `/Game/CastleFortress/Blueprints/Controllers/AIController_Generic` OwnerActor))
    (bind _output_get (set `self.AIConRef` _asaicontroller_generic)))
  (if (not (!= (`self.CharRef`) null))
    (bind _ascharacter_paladin (cast `/Game/CastleFortress/Blueprints/Characters/Character_Paladin` (`Controller.K2_GetPawn` _aiconref)))
    (set `self.CharRef` _ascharacter_paladin))
  (`/Engine/EditorBlueprintResources/StandardMacros.IsValid` (`BTFunctionLibrary.GetBlackboardValueAsActor` (`self.TargetActor`))
    (:`Is Valid`
      (`/Game/CastleFortress/Blueprints/Controllers/AIController_Generic.AttackStart` _output_get (`BTFunctionLibrary.GetBlackboardValueAsFloat` (`self.TargetHealth`))))
    (:`Is Not Valid`
      (`/Game/CastleFortress/Blueprints/Controllers/AIController_Generic.AttackStop` _output_get)))
  (`self.FinishExecute` true))

(fn `EndAttackPose`
  (message `/Game/Caladan/Blueprint/MyInterface.InterfaceAttackPoseEnd` (`SkeletalMeshComponent.GetAnimInstance` (`Character.Mesh` (`self.CharRef`)))))