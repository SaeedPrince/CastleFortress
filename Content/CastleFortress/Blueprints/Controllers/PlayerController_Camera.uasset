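; Player controller that toggles between direct character control and a strategy-style camera pawn with movement, rotation and zoom.
; In camera mode an AI controller possesses the player's character, which can be selected under the cursor and sent to clicked Landscape points.
; Looping timers step movement and turning toward the target without pathfinding; five earlier movement algorithms remain disconnected in MoveToward.
; Debug-style inputs ask the game mode to add random allies or enemies.
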(event `self.ReceiveBeginPlay`
  ;[0 1 0] Begin Play
  (bind _asgame_mode_generic (cast `/Game/CastleFortress/Blueprints/GameModes/GameMode_Generic` (`GameplayStatics.GetGameMode`)))
  (bind _output_get (set `self.GameModeRef` _asgame_mode_generic))
  (set `self.GameStateRef` (`/Game/CastleFortress/Blueprints/GameModes/GameMode_Generic.GameStateRef` _output_get)))

(event `self.ReceiveTick`
  (params (DeltaSeconds :type "Float (single-precision)"))
  (bind (_bblockinghit _binitialoverlap _time _location _impactpoint _normal _impactnormal _physmat _hitactor) (`GameplayStatics.BreakHitResult` (`self.GetHitResultUnderCursorForObjects` (`|MakeArray` "ObjectTypeQuery3" :!type "EObjectTypeQuery Enum"))))
  ;[1 1 0] Checks if mouse is on character
  (if (`self.IsCameraActive`)
    (if (== (`GameplayStatics.GetObjectClass` _hitactor) "/Game/CastleFortress/Blueprints/Characters/Paladin_Player.Paladin_Player_C")
      (set `self.CurrentMouseCursor` "Crosshairs")
      (bind _ascharacter_paladin (cast `/Game/CastleFortress/Blueprints/Characters/Character_Paladin` _hitactor))
      (set `self.CharacterUnderCursor` _ascharacter_paladin)
      (else
        (set `self.CurrentMouseCursor` "Default")))))

(event `InputAction|ChangeCamera`
  (params (Key :type "Key Structure"))
  ;[1 1 0] Change Camera
  (:`Pressed`
    (bind (_self _outputpawn) (`self.ChangeCamera`))
    (`self.Possess` _self _outputpawn)))

(event `InputAxis|MoveForward` :overrideparent false
  (params (AxisValue :type "Float (single-precision)"))
  ;[1 1 0] Movement
  (`/Engine/EditorBlueprintResources/StandardMacros.IsValid` (`self.CurrentPawn`)
    (:`Is Valid`
      (`self.MovePawn` AxisValue "Forward"))))

(event `InputAxis|MoveRight` :overrideparent false
  (params (AxisValue :type "Float (single-precision)"))
  ;[1 1 0] Movement
  (`/Engine/EditorBlueprintResources/StandardMacros.IsValid` (`self.CurrentPawn`)
    (:`Is Valid`
      (`self.MovePawn` AxisValue "Right"))))

(event `InputAction|Attack-Select`
  (params (Key :type "Key Structure"))
  ;[1 1 0] Select / Deselect
  (:`Pressed`
    (if (`self.IsCameraActive`)
      (if (`|EnumEquality` (`self.CurrentMouseCursor`) "Crosshairs")
        (`KismetSystemLibrary.PrintString` "Character is selected")
        (set `self.IsCharacterSelected` true)
        (set `self.CharacterSelected` (`self.CharacterUnderCursor`))
        (else
          (`KismetSystemLibrary.PrintString` "Nothing is selected")
          (set `self.IsCharacterSelected` false)
          (set `self.CharacterSelected` (`self.CharacterNull`)))))))

(event `InputAction|MoveToPoint`
  (params (Key :type "Key Structure"))
  (bind (_bblockinghit _binitialoverlap _time _location _impactpoint _normal _impactnormal _physmat _hitactor) (`GameplayStatics.BreakHitResult` (`self.GetHitResultUnderCursorForObjects` (`|MakeArray` "ObjectTypeQuery1" :!type "EObjectTypeQuery Enum"))))
  ;[1 1 0] Move to point
  (:`Pressed`
    (`/Engine/EditorBlueprintResources/StandardMacros.IsValid` (`self.CharacterSelected`)
      (:`Is Valid`
        (if (`self.IsCameraActive`)
          (`self.SetPointsToGo` _hitactor _location)
          (bind _returnvalue (`KismetSystemLibrary.K2_SetTimer` self "MoveToward" (`self.MoveFrequency`) true))
          (set `self.TimerMoveToward` _returnvalue)
          (set `self.StartingPoint` (`self.K2_GetActorLocation` (`self.CharacterMoveToward`)))
          (bind _returnvalue_2 (`KismetSystemLibrary.K2_SetTimer` self "TurnToward" (`self.TurnFrequency`) true))
          (set `self.TimerTurnToward` _returnvalue_2))))))

(event `InputAction|AddAlly`
  (params (Key :type "Key Structure"))
  ;[1 1 0] Adds an ally AI
  (:`Pressed`
    (`/Game/CastleFortress/Blueprints/GameModes/GameMode_Generic.AddAIRandom` (`self.GameModeRef`) "Ally")))

(event `InputAction|AddEnemy`
  (params (Key :type "Key Structure"))
  ;[1 1 0] Adds an ally AI
  (:`Pressed`
    (`/Game/CastleFortress/Blueprints/GameModes/GameMode_Generic.AddAIRandom` (`self.GameModeRef`) "Enemy")))

(event `InputAxis|CameraRotation`
  (params (AxisValue :type "Float (single-precision)"))
  (bind _springarmref (`self.SpringArmRef`))
  ;[1 1 0] Camera Rotation
  (`/Engine/EditorBlueprintResources/StandardMacros.IsValid` _springarmref
    (:`Is Valid`
      (`SceneComponent.K2_SetWorldRotation` _springarmref (`KismetMathLibrary.MakeRotator` (.roll (`SceneComponent.K2_GetComponentRotation` _springarmref)) (.pitch (`SceneComponent.K2_GetComponentRotation` _springarmref)) (+ (.yaw (`SceneComponent.K2_GetComponentRotation` _springarmref)) AxisValue)) false false))))

(event `InputAxis|CameraZoom`
  (params (AxisValue :type "Float (single-precision)"))
  (bind (_currentrotator_roll _currentrotator_pitch _currentrotator_yaw) (`KismetMathLibrary.BreakRotator` (`self.CurrentRotator`)))
  (bind _springarmref (`self.SpringArmRef`))
  (bind _returnvalue (* AxisValue (`self.CameraAdjustment`)))
  ;[1 1 0] Camera Zoom
  (if (`self.IsCameraActive`)
    (`SceneComponent.K2_SetWorldLocation` _springarmref (`KismetMathLibrary.MakeVector` (- (.x (`SceneComponent.K2_GetComponentLocation` _springarmref)) _returnvalue) (+ (.y (`SceneComponent.K2_GetComponentLocation` _springarmref)) (* _returnvalue _currentrotator_yaw)) (+ (.z (`SceneComponent.K2_GetComponentLocation` _springarmref)) _returnvalue)) false false)))

(fn `MovePawn`
  (params (AxisValue :type "Float (double-precision)") (MoveDirection :type String))
  (if (`self.IsCameraActive`)
    (`/Game/CastleFortress/Blueprints/Pawns/Pawn_Camera.Move` (`self.CameraRef`) AxisValue MoveDirection)
    (else
      (`/Game/CastleFortress/Blueprints/Characters/Character_Paladin.MoveByInput` (`self.CharacterRef`) AxisValue MoveDirection))))

(fn `MoveToward`
  (bind (_outputbool _movement) (`/Game/CastleFortress/Blueprints/Characters/Character_Paladin.FarAwayXY` (`self.CharacterMoveToward`) (`self.EndPoint`)))
  ;[0 1 0] Sixth Algorithm
  (if (!= (`self.XDistribution`) -1.0)
    (if _outputbool
      (`/Game/CastleFortress/Blueprints/Controllers/AIController_Generic.MoveDirectly` (`self.AI_GenericRef`) _movement)
      (else
        (`KismetSystemLibrary.K2_ClearAndInvalidateTimerHandle` (`self.TimerMoveToward`) :!label _label)))
    (else
      (goto _label))))

(fn `SetCurrentRotator`
  (if (`self.IsCameraActive`)
    (set `self.CurrentRotator` (`self.K2_GetActorRotation` (`self.CurrentPawn`)))
    (else
      (set `self.CurrentRotator` (`Pawn.GetControlRotation` (`self.CurrentPawn`))))))

(fn `TurnToward`
  (locals (LocalAxis :type "Float (double-precision)"))
  (bind (_outputbool _clockwise) (`/Game/CastleFortress/Blueprints/Characters/Character_Paladin.IsLookingAtPoint` (`self.CharacterMoveToward`) (`self.EndPoint`) (`self.StartingPoint`)))
  (if _outputbool
    (`KismetSystemLibrary.K2_ClearAndInvalidateTimerHandle` (`self.TimerTurnToward`))
    (else
      (`/Game/CastleFortress/Blueprints/Controllers/AIController_Generic.TurnByInput` (`self.AI_GenericRef`) _clockwise))))

(fn `UserConstructionScript`)