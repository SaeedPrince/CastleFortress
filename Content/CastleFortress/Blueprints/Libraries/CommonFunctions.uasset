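; Blueprint function library of shared math, rotation, spawn transform, randomization and distance helpers for CastleFortress.
; Vector helpers derive movement axes and 2D or atan2-based angles, alongside sign, integer power and random array picks.
; IsCharacterFacingToActor compares the flattened angle between actor direction and capsule forward, yawed 25 degrees, returning true above the threshold despite its name.
; RandomIntegersFromTwoArrays bounds both random indices by the first array's length.
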(fn `AFloatPowerBInt`
  (params (InputA :type "Float (double-precision)") (InputB :type Integer))
  (returns (OutputFloat :type "Float (double-precision)"))
  (locals (OutFloat :type "Float (double-precision)" :default 1.0) (Counter :type Integer))
  (bind _output_get (set `local.Counter` InputB))
  (while (> _output_get 0)
    (set `local.OutFloat` (* InputA (`local.OutFloat`)))
    (set `local.Counter` (- (`local.Counter`) 1)))
  (return (`local.OutFloat`)))

(fn `AngleBetweenVectors2D`
  (params (VectorA :type "Vector Structure") (VectorB :type "Vector Structure"))
  (returns (OutputAngle :type "Float (double-precision)"))
  (return (`KismetMathLibrary.DegAcos` (`KismetMathLibrary.Dot_VectorVector` (`KismetMathLibrary.Normal` (`KismetMathLibrary.MakeVector` (.x VectorA) (.y VectorA))) (`KismetMathLibrary.Normal` (`KismetMathLibrary.MakeVector` (.x VectorB) (.y VectorB)))))))

(fn `AngleFromPerp`
  (params (VectorA :type "Vector Structure") (VectorB :type "Vector Structure"))
  (returns (AngleDegree :type "Float (double-precision)"))
  (return (`KismetMathLibrary.DegAtan2` (`self.Perp` VectorA VectorB) (`KismetMathLibrary.Dot_VectorVector` VectorA VectorB))))

(fn `DestinationBetweenTwoActors`
  (params (Actor1 :type "Actor Object Reference") (Actor2 :type "Actor Object Reference"))
  (returns (Destination :type "Float (double-precision)"))
  (return (`KismetMathLibrary.VSize` (- (`Actor.K2_GetActorLocation` Actor1) (`Actor.K2_GetActorLocation` Actor2)))))

(fn `GetDirectionFromScenceComponent`
  (params (ScenceComponent :type "SceneComponent Object Reference"))
  (returns (Direction :type "Vector Structure"))
  (return (`KismetMathLibrary.Conv_RotatorToVector` (`KismetMathLibrary.MakeRotator` (.roll (`SceneComponent.K2_GetComponentRotation` ScenceComponent)) (.pitch (`SceneComponent.K2_GetComponentRotation` ScenceComponent)) (+ (.yaw (`SceneComponent.K2_GetComponentRotation` ScenceComponent)) 25.0)))))

(fn `GetMovementVector`
  (params (Rotator :type "Rotator Structure") (Direction :type String))
  (returns (OutVector :type "Vector Structure"))
  (locals (OutVect :type "Vector Structure"))
  (switch `string` Direction
    (:`Forward`
      (set `local.OutVect` (`KismetMathLibrary.GetForwardVector` Rotator)))
    (:`Right`
      (set `local.OutVect` (`KismetMathLibrary.GetRightVector` Rotator))))
  (return (`local.OutVect`)))

(fn `IsCharacterFacingToActor`
  (params (ActorLocation :type "Vector Structure") (Character :type "Character Object Reference") (AcceptableAngle :type "Float (double-precision)"))
  (returns (Output :type Boolean))
  (return (> (`self.AngleBetweenVectors2D` (- ActorLocation (`Actor.K2_GetActorLocation` Character)) (`self.GetDirectionFromScenceComponent` (`Character.CapsuleComponent` Character))) AcceptableAngle)))

(fn `MakeRotatorByZ`
  (params (InputRotator :type "Rotator Structure"))
  (returns (OutputRotator :type "Rotator Structure"))
  (return (`KismetMathLibrary.MakeRotator` 0.0 0.0 (.yaw InputRotator))))

(fn `MakeSpawnTransform`
  (params (InputActor :type "Actor Object Reference"))
  (returns (OutputTransform :type "Transform Structure"))
  (return (`KismetMathLibrary.MakeTransform` (.location (`Actor.GetTransform` InputActor)) (.rotation (`Actor.GetTransform` InputActor)))))

(fn `Perp`
  (params (VectorA :type "Vector Structure") (VectorB :type "Vector Structure"))
  (returns (OutputFloat :type "Float (double-precision)"))
  (return (* (`KismetMathLibrary.DegTan` (`KismetMathLibrary.DegAcos` (`KismetMathLibrary.Dot_VectorVector` (`KismetMathLibrary.Normal` (`KismetMathLibrary.MakeVector` (.x VectorA) (.y VectorA))) (`KismetMathLibrary.Normal` (`KismetMathLibrary.MakeVector` (.x VectorB) (.y VectorB)))))) (`KismetMathLibrary.Dot_VectorVector` VectorA VectorB))))

(fn `RandomIntegerFromArray`
  (params (InputArray :type "Array of Integer"))
  (returns (OutInteger :type Integer))
  (return (`|GetArrayItem` InputArray (`KismetMathLibrary.RandomInteger` (`KismetArrayLibrary.Array_Length` InputArray)))))

(fn `RandomIntegersFromTwoArrays`
  (params (Array1 :type "Array of Integer") (Array2 :type "Array of Integer"))
  (returns (Value1 :type Integer) (Value2 :type Integer))
  (bind _returnvalue (`KismetMathLibrary.RandomIntegerInRange` 0 (- (`KismetArrayLibrary.Array_Length` Array1) 1)))
  (return (`|GetArrayItem` Array1 _returnvalue) (`|GetArrayItem` Array2 _returnvalue)))

(fn `RandomIntRangePositiveOrNegative`
  (params (Min :type Integer) (Max :type Integer))
  (returns (ReturnValue :type Integer))
  (return (* (`KismetMathLibrary.RandomIntegerInRange` Min Max) (`self.RandomIntegerFromArray` (`|MakeArray` 1 -1)))))

(fn `Sgn`
  (params (InputFloat :type "Float (double-precision)"))
  (returns (OutputFloat :type "Float (double-precision)"))
  (locals (OutFloat :type "Float (double-precision)"))
  (if (> InputFloat 0.0)
    (set `local.OutFloat` 1.0)
    (elif (< InputFloat 0.0)
      (set `local.OutFloat` -1.0)))
  (return (`local.OutFloat`)))