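; Game_Caladan is the game-level manager that admits players and spawns their characters.
; InitializeGame records the level name and caches every PlayerStart transform.
; CreateNewCharacter rejects already-registered names, except "Default Player", then assigns the Footman controller a capped, incrementing player index.
; That index selects the start transform for an authority-only spawn and possess; AssignHud is an empty stub.
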(fn `AddPlayerName`
  (params (InputName :type String))
  (bind _outputboolean (`self.IsStringInStringArray` (`self.PlayerNameArray`) InputName))
  (if (not _outputboolean)
    (`KismetArrayLibrary.Array_Add` (`self.PlayerNameArray`) InputName)))

(fn `AssignHud`)

(fn `CreateNewCharacter`
  (params (InputController :type "PlayerController Object Reference") (InputCharacter :type "/Game/Caladan/Blueprint/Character_Footman Class Reference") (InputName :type String))
  (returns (OutputCharacter :type "Character Object Reference"))
  (if (`KismetStringLibrary.NotEqual_StrStr` InputName "Default Player")
    (bind _outputboolean (`self.IsStringInStringArray` (`self.PlayerNameArray`) InputName))
    (if (not _outputboolean)
      (`/Engine/EditorBlueprintResources/StandardMacros.IsValid` InputController :!label _label
        (:`Is Valid`
          (bind _ascontroller_footman (cast `/Game/Caladan/Blueprint/Controller_Footman` InputController))
          (bind (_creationallowed _playerindex) (`self.CreateNewPlayerIndex`))
          (if _creationallowed
            (bind _output_get (set `/Game/Caladan/Blueprint/Controller_Footman.PlayerIndex` _playerindex _ascontroller_footman))
            (bind _outputcharacter (`self.SpawnCharacter` InputController _output_get InputCharacter))
            (`self.AssignHud`)
            (return _outputcharacter)
            (else
              (`KismetSystemLibrary.PrintString` "No new player allowed" true false (struct :`G` 0.66 :`B` 1.0 :`A` 1.0) 8.0))))))
    (else
      (goto _label))))

(fn `CreateNewPlayerIndex`
  (returns (CreationAllowed :type Boolean) (PlayerIndex :type Integer))
  (bind _returnvalue (<= (`self.PlayerCountNum`) (`self.PlayerMaxAllowed`)))
  (if _returnvalue
    (bind _output_get (set `self.PlayerCountNum` (+ (`self.PlayerCountNum`) 1)))
    (return _returnvalue (- _output_get 1))))

(fn `CreatePlayerStartArray`
  (bind _outactors (`GameplayStatics.GetAllActorsOfClass` "/Script/Engine.PlayerStart"))
  (for _array_element _outactors
    (`KismetArrayLibrary.Array_Add` (`self.CharacterStart`) (`self.GetTransform` _array_element))))

(fn `InitializeGame`
  (`self.InitializeMap`)
  (`self.CreatePlayerStartArray`))

(fn `InitializeMap`
  (bind _returnvalue (`GameplayStatics.GetCurrentLevelName` true))
  (set `self.LevelPlaying` _returnvalue))

(fn `IsStringInStringArray`
  (params (InputArray :type "Array of String") (InputString :type String))
  (returns (OutputBoolean :type Boolean))
  (locals (LocalOutput :type Boolean))
  (for _array_element InputArray
    (if (`KismetStringLibrary.EqualEqual_StrStr` _array_element InputString)
      (set `local.LocalOutput` true)
      (break)))
  (return (`local.LocalOutput`)))

(fn `SpawnCharacter`
  (params (InputController :type "PlayerController Object Reference") (InputIndex :type Integer) (InputCharacter :type "/Game/Caladan/Blueprint/Character_Footman Class Reference"))
  (returns (OutputCharacter :type "Character Object Reference"))
  (locals (LocalInputController :type "PlayerController Object Reference") (LocalInputIndex :type Integer) (LocalSpawnResult :type "/Game/Caladan/Blueprint/Character_Footman Object Reference") (LocalCharacter :type "/Game/Caladan/Blueprint/Character_Footman Class Reference"))
  (`/Engine/EditorBlueprintResources/StandardMacros.IsValid` InputController
    (:`Is Valid`
      (`/Engine/EditorBlueprintResources/ActorMacros.Switch Has Authority`
        (:`Authority`
          (bind _returnvalue (`|SpawnActorFromClass` InputCharacter (`|GetArrayItem` (`self.CharacterStart`) InputIndex) "Undefined" "OverrideRootScale" InputController null))
          (bind _output_get (set `local.LocalSpawnResult` _returnvalue))
          (`/Engine/EditorBlueprintResources/StandardMacros.IsValid` _output_get
            (:`Is Valid`
              (`Controller.Possess` InputController _returnvalue)
              (bind _output_get_2 (set `/Game/Caladan/Blueprint/Character_Footman.MyIndex` InputIndex _returnvalue))
              (`KismetArrayLibrary.Array_Add` (`/Game/Caladan/Blueprint/Character_Footman.ViewIndex` _returnvalue) _output_get_2)
              (return _returnvalue))))))))

(fn `UserConstructionScript`)