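; TheGameInstance is a game instance Blueprint that stores the player's name and controls music playback.
; SetPlayerName writes the input to PlayerName, with a debug print left disconnected.
; InitSound assigns the Ascension track to the Sound audio component and places it at the world origin.
; PlayMusic and StopMusic then start that component from the beginning or stop it.
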(fn `InitSound`
  (bind _sound (`self.Sound`))
  (`AudioComponent.SetSound` _sound "/Game/Caladan/Audio/Music/SOZ073_01-Ascension_Full.SOZ073_01-Ascension_Full")
  (`SceneComponent.K2_SetWorldLocation` _sound (0.0 0.0 0.0) false false))

(fn `PlayMusic`
  (`AudioComponent.Play` (`self.Sound`) 0.0))

(fn `SetPlayerName`
  (params (InputName :type String))
  (set `self.PlayerName` InputName))

(fn `StopMusic`
  (`AudioComponent.Stop` (`self.Sound`)))