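; Player controller for the Footman character in the Caladan game, handling character spawning, attack/block input and the player's UI.
; A spawn request has the Game_Caladan game mode create the character and record the player name, then links pawn and controller.
; Fire and Block use press-to-pose, release-to-act requests, each cancelling the other on the character.
; A Health RepNotify updates the local healthbar; BeginPlay is empty, leaving the client HUD setup function uncalled here.
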(event `self.ReceiveBeginPlay`
  ;[1 1 1] Begin Play
)

(event `RequestSpawnCharacterOnServer`
  (params (InputClass :type "/Game/Caladan/Blueprint/Character_Footman Class Reference") (InputPlayer :type String))
  ;[1 1 1] Spawn Character
  (set `self.PlayerName` InputPlayer)
  (bind _asgame_caladan (cast `/Game/Caladan/Blueprint/Game_Caladan` (`GameplayStatics.GetGameMode`)))
  (bind _outputcharacter (`/Game/Caladan/Blueprint/Game_Caladan.CreateNewCharacter` _asgame_caladan self InputClass InputPlayer))
  (`/Game/Caladan/Blueprint/Game_Caladan.AddPlayerName` _asgame_caladan InputPlayer)
  (bind _ascharacter_footman (cast `/Game/Caladan/Blueprint/Character_Footman` _outputcharacter))
  (`/Engine/EditorBlueprintResources/StandardMacros.IsValid` _ascharacter_footman
    (:`Is Valid`
      (bind _output_get (set `self.CharacterBP` _ascharacter_footman))
      (set `/Game/Caladan/Blueprint/Character_Footman.TheController` self _output_get))))

(event `InputAction|Fire`
  (params (Key :type "Key Structure"))
  (bind _characterbp (`self.CharacterBP`))
  ;[1 1 1] Fire Start
  (:`Pressed`
    (`/Engine/EditorBlueprintResources/StandardMacros.IsValid` _characterbp
      (:`Is Valid`
        (if (`/Game/Caladan/Blueprint/Character_Footman.IsDefendPressed` _characterbp)
          (`/Game/Caladan/Blueprint/Character_Footman.RequestDefendReleaseOnServer` _characterbp))
        (`self.RequestAttackPoseOnServer`))))
  (:`Released`
    (`/Engine/EditorBlueprintResources/StandardMacros.IsValid` _characterbp
      (:`Is Valid`
        (if (`/Game/Caladan/Blueprint/Character_Footman.IsFirePressed` (`self.CharacterBP`))
          (set `/Game/Caladan/Blueprint/Character_Footman.IsFireInProgress` true (`self.CharacterBP`))
          (`self.RequestAttackExeOnServer`))))))

(event `RequestAttackPoseOnServer`
  (bind _characterbp (`self.CharacterBP`))
  ;[1 1 1] Fire Start
  (set `/Game/Caladan/Blueprint/Character_Footman.IsFirePressed` true _characterbp)
  (set `/Game/Caladan/Blueprint/Character_Footman.IsFireReleased` false _characterbp))

(event `RequestAttackExeOnServer`
  (bind _characterbp (`self.CharacterBP`))
  ;[1 1 1] Fire Start
  (set `/Game/Caladan/Blueprint/Character_Footman.IsFirePressed` false _characterbp)
  (set `/Game/Caladan/Blueprint/Character_Footman.IsFireReleased` true _characterbp))

(event `InputAction|Block`
  (params (Key :type "Key Structure"))
  (bind _characterbp (`self.CharacterBP`))
  ;[1 1 1] Defend
  (:`Pressed`
    (`/Engine/EditorBlueprintResources/StandardMacros.IsValid` _characterbp
      (:`Is Valid`
        (if (`/Game/Caladan/Blueprint/Character_Footman.IsFirePressed` _characterbp)
          (`/Game/Caladan/Blueprint/Character_Footman.RequestAttackEndOnServer` _characterbp))
        (`/Game/Caladan/Blueprint/Character_Footman.RequestDefendPoseOnServer` _characterbp))))
  (:`Released`
    (`/Game/Caladan/Blueprint/Character_Footman.RequestDefendReleaseOnServer` _characterbp)))

(fn `AdjustHealthbar`
  (if (`self.IsLocalController` self)
    (`ProgressBar.SetPercent` (`/Game/Caladan/Blueprint/Healthbar.HealthSelf` (`self.HealthBar`)) (`self.Health`))))

(fn `BeginPlayOnClient`
  (`self.CreateHud`)
  (`self.CursorHide`)
  (`self.SetGameMode`)
  (`self.CreateHealthbar`)
  (`self.AdjustHealthbar`))

(fn `CreateHealthbar`
  (if (`self.IsLocalPlayerController` self)
    (bind _returnvalue (`|CreateWidget` "/Game/Caladan/Blueprint/Healthbar.Healthbar_C" self))
    (`/Engine/EditorBlueprintResources/StandardMacros.IsValid` _returnvalue
      (:`Is Valid`
        (`UserWidget.AddToViewport` _returnvalue 0)
        (bind _output_get (set `self.HealthBar` _returnvalue))
        (`TextBlock.SetText` (`/Game/Caladan/Blueprint/Healthbar.txtNameSelf` _output_get) (`KismetTextLibrary.Conv_StringToText` (`self.PlayerName`))))
      (:`Is Not Valid`
        (`KismetSystemLibrary.PrintString` "Healthbar invalid" true false (struct :`G` 0.66 :`B` 1.0 :`A` 1.0) 8.0)))))

(fn `CreateHud`
  (bind _ashud_footman (cast `/Game/Caladan/Blueprint/Hud_Footman` (`self.GetHUD`)))
  (set `self.HudObject` _ashud_footman))

(fn `CursorHide`
  (set `self.bShowMouseCursor` false))

(fn `CursorShow`
  (set `self.bShowMouseCursor` true))

(fn `OnRep_Health`
  (`self.AdjustHealthbar`))

(fn `SetGameInstance`
  (returns (OutputPlayer :type String))
  (bind _asthe_game_instance (cast `/Game/Caladan/Blueprint/TheGameInstance` (`GameplayStatics.GetGameInstance`)))
  (`/Engine/EditorBlueprintResources/StandardMacros.IsValid` _asthe_game_instance
    (:`Is Valid`
      (bind _output_get (set `self.GameInstance` _asthe_game_instance))
      (bind _playername (`/Game/Caladan/Blueprint/TheGameInstance.PlayerName` _output_get))
      (if (`KismetStringLibrary.NotEqual_StrStr` _playername)
        (return _playername)))))

(fn `SetGameMode`
  (bind _asgame_caladan (cast `/Game/Caladan/Blueprint/Game_Caladan` (`GameplayStatics.GetGameMode`)))
  (set `self.TheGameMode` _asgame_caladan))

(fn `SpawnCharacter`
  (if (`self.IsLocalPlayerController` self)
    (`self.RequestSpawnCharacterOnServer` "/Game/Caladan/Footman/Blueprint/Character_Footman_male.Character_Footman_male_C")
    (else
      (`self.RequestSpawnCharacterOnServer` "/Game/Caladan/Maria/Blueprint/Character_Footman_female.Character_Footman_female_C"))))

(fn `UserConstructionScript`)